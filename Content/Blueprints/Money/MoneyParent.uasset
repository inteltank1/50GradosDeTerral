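; Money pickup, apparently a base class for variants, that adds its value to the player's money when touched.
; BeginPlay caches the PL_MainCharacter, and Tick rotates the root toward it so the plane works as a billboard.
; When that character class overlaps the box, it spawns a particle system, adds Moneyitgives to Money, calls SetMoney on the character and destroys itself.
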(event OnComponentBeginOverlap(Box)
  (params (OverlappedComponent :type Primitive%20Component%20Object%20Reference) (OtherActor :type Actor%20Object%20Reference) (OtherComp :type Primitive%20Component%20Object%20Reference) (OtherBodyIndex :type Integer) (bFromSweep :type Boolean) (SweepResult :type Hit%20Result%20Structure%20%28by%20ref%29))
  (if (Utilities|ClassIsChildOf (Utilities|GetClass OtherActor) "/Game/Blueprints/CharacterAndControls/PL_MainCharacter.PL_MainCharacter_C")
    (Niagara|SpawnSystematLocation (Variables|Default|GetParticle) (Transformation|GetActorLocation))
    (bind _aspl_main_character (Utilities|Casting|CastToPL_MainCharacter OtherActor))
    (Variables|/Game/Blueprints/CharacterAndControls/PL_MainCharacter.PL_MainCharacter_C|SetMoney _aspl_main_character (+ (Variables|/Game/Blueprints/CharacterAndControls/PL_MainCharacter.PL_MainCharacter_C|GetMoney _aspl_main_character) (Variables|Default|GetMoneyitgives)))
    (Default|SetMoney _aspl_main_character)
    (Actor|DestroyActor)))

(event EventBeginPlay
  (bind _returnvalue (Actor|GetActorOfClass "/Game/Blueprints/CharacterAndControls/PL_MainCharacter.PL_MainCharacter_C"))
  (bind _aspl_main_character (Utilities|Casting|CastToPL_MainCharacter _returnvalue))
  (Variables|Default|SetAs%20PL%20Main%20Character _aspl_main_character))

(event Collision|EventActorBeginOverlap
  (params (OtherActor :type Actor%20Object%20Reference)))

(event EventTick
  (params (DeltaSeconds :type Float%20%28single-precision%29))
  ;[1 1 1] Always Face Player
  (Transformation|SetWorldRotation (Variables|Default|GetDefaultSceneRoot) (Math|Rotator|FindLookatRotation (Transformation|GetWorldLocation (Variables|Default|GetPlane)) (Transformation|GetActorLocation (Variables|Default|GetAs%20PL%20Main%20Character))) false false))

(fn ConstructionScript)