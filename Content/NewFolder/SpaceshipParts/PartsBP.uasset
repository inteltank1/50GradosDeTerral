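; Collectible spaceship part pickup whose plane material is picked by a Number in the construction script.
; On Tick it turns to face the first-person character, cached on BeginPlay, and drives a delay-loop macro that repeatedly spawns doubled fireworks, which also fire at start.
; When the character overlaps it, it increments their NumberOfParts, calls Illocambiate, spawns a pickup effect and destroys itself.
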(event OnComponentBeginOverlap(r)
  (params (OverlappedComponent :type Primitive%20Component%20Object%20Reference) (OtherActor :type Actor%20Object%20Reference) (OtherComp :type Primitive%20Component%20Object%20Reference) (OtherBodyIndex :type Integer) (bFromSweep :type Boolean) (SweepResult :type Hit%20Result%20Structure%20%28by%20ref%29))
  (bind _as_bp_first_person_character (Variables|Default|GetAs%20BP%20First%20Person%20Character))
  (bind _niagara (Variables|Default|GetNiagara))
  (if (Utilities|ClassIsChildOf (Utilities|GetClass OtherActor) "/Game/FirstPerson/Blueprints/BP_FirstPersonCharacter.BP_FirstPersonCharacter_C")
    (Math|Integer|IncrementInt (Variables|/Game/FirstPerson/Blueprints/BP_FirstPersonCharacter.BP_FirstPersonCharacter_C|GetNumberOfParts _as_bp_first_person_character)
      (:%20%20
        (Default|Illocambiate _as_bp_first_person_character)
        (Niagara|SpawnSystematLocation "/Game/NewFolder/SpaceshipParts/RocketPickUp.RocketPickUp" (Transformation|GetWorldLocation _niagara) (Transformation|GetWorldRotation _niagara))
        (Actor|DestroyActor)))))

(event EventBeginPlay
  (bind _returnvalue (Transformation|GetActorLocation))
  (Utilities|FlowControl|Sequence
    (:then_0
      (bind _returnvalue_2 (Actor|GetActorOfClass "/Game/FirstPerson/Blueprints/BP_FirstPersonCharacter.BP_FirstPersonCharacter_C"))
      (bind _asbp_first_person_character (Utilities|Casting|CastToBP_FirstPersonCharacter _returnvalue_2))
      (Variables|Default|SetAs%20BP%20First%20Person%20Character _asbp_first_person_character))
    (:then_1
      (Niagara|SpawnSystematLocation "/Game/NewFolder/Mapas/MuelleUno/FireworksFolder/Fireworks2.Fireworks2" _returnvalue)
      (Niagara|SpawnSystematLocation "/Game/NewFolder/Mapas/MuelleUno/FireworksFolder/Fireworks2.Fireworks2" _returnvalue))))

(event Collision|EventActorBeginOverlap
  (params (OtherActor :type Actor%20Object%20Reference)))

(event EventTick
  (params (DeltaSeconds :type Float%20%28single-precision%29))
  (bind _returnvalue (Transformation|GetActorLocation))
  (Transformation|SetActorRotation (Math|Rotator|FindLookatRotation (Transformation|GetActorLocation) (Transformation|GetActorLocation (Variables|Default|GetAs%20BP%20First%20Person%20Character))))
  (Utilities|LoopwithDelay true 5.0
    (:Loop%20Body
      (Niagara|SpawnSystematLocation "/Game/NewFolder/Mapas/MuelleUno/FireworksFolder/Fireworks2.Fireworks2" _returnvalue)
      (Niagara|SpawnSystematLocation "/Game/NewFolder/Mapas/MuelleUno/FireworksFolder/Fireworks2.Fireworks2" _returnvalue))))

(fn ConstructionScript
  (bind _plane (Variables|Default|GetPlane))
  (switch int (Variables|Default|GetNumber)
    (:0
      (Rendering|Material|SetMaterial _plane 0 "/Game/NewFolder/SpaceshipParts/Mats/toppart_Mat.toppart_Mat"))
    (:1
      (Rendering|Material|SetMaterial _plane 0 "/Game/NewFolder/SpaceshipParts/Mats/Legs_Mat.Legs_Mat"))
    (:2
      (Rendering|Material|SetMaterial _plane 0 "/Game/NewFolder/SpaceshipParts/Mats/LowerPartBody_Mat.LowerPartBody_Mat"))
    (:3
      (Rendering|Material|SetMaterial _plane 0 "/Game/NewFolder/SpaceshipParts/Mats/Toppartbody_Mat.Toppartbody_Mat"))
    (:4
      (Rendering|Material|SetMaterial _plane 0 "/Game/NewFolder/SpaceshipParts/Mats/Windows_Mat.Windows_Mat"))))